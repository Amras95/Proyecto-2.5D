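; Moving platform that shuttles back and forth in a straight line between its starting position and a point Distance units along Direction.
; BeginPlay stores the start point, then nudges the platform just outside the endpoint tolerance so it does not reverse immediately.
; Each Tick, Movement applies a delta-time-scaled, unswept location change, then CheckLimits tests proximity to either endpoint and Speed flips sign on a hit.
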(event `self.ReceiveBeginPlay`
  (set `self.Inicpos` (`self.K2_GetActorLocation`))
  (`self.K2_SetActorLocation` (+ (`self.K2_GetActorLocation`) (* (`KismetMathLibrary.Normal` (`self.Direction`)) 15.0))))

(event `self.ReceiveTick`
  (params (DeltaSeconds :type "Float (single-precision)"))
  (`self.Movement`)
  (bind _limitchecked (`self.CheckLimits`))
  (if _limitchecked
    (set `self.Speed` (* (`self.Speed`) -1.0))))

(fn `CheckLimits`
  (returns (LimitChecked :type Boolean))
  (if (or (<= (`KismetMathLibrary.Vector_Distance` (`self.Inicpos`) (`self.K2_GetActorLocation`)) 10.0) (<= (`KismetMathLibrary.Vector_Distance` (+ (`self.Inicpos`) (* (`KismetMathLibrary.Normal` (`self.Direction`)) (`self.Distance`))) (`self.K2_GetActorLocation`)) 10.0))
    (return true)
    (else
      (return false))))

(fn `Movement`
  (`self.K2_SetActorLocation` (+ (`self.K2_GetActorLocation`) (* (`KismetMathLibrary.Normal` (`self.Direction`)) (* (`self.Speed`) (`GameplayStatics.GetWorldDeltaSeconds`))))))

(fn `UserConstructionScript`)