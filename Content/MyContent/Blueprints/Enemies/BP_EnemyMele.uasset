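; Melee enemy that patrols platforms along the X axis and damages the Soldier on overlap.
; Each Tick, downward traces at both capsule edges detect ledges, flipping speed and rotation while patrolling.
; A sphere trace detects the Soldier and an eye-level trace checks line of sight.
; With the Soldier visible, it keeps moving in its facing direction but stops at the ledge ahead instead of turning.
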(event `self.ReceiveBeginPlay`
  ;[1 1 1] Set Default Speed
  (set `self.defaultSpeed` (`self.speed`)))

(event `self.ReceiveTick`
  (params (DeltaSeconds :type "Float (single-precision)"))
  (bind (_returnvalue_roll _returnvalue_pitch _returnvalue_yaw) (`KismetMathLibrary.BreakRotator` (`self.GetControlRotation`)))
  (bind (_returnvalue_roll_2 _returnvalue_pitch_2 _returnvalue_yaw_2) (`KismetMathLibrary.BreakRotator` (`self.GetControlRotation`)))
  ;[1 1 1] Patrolling
  (bind (_detected _character) (`self.CheckCharacter`))
  (if _detected
    (bind _detected_2 (`self.CheckVision` _character))
    (if _detected_2
      (`self.GetDirection`)
      (bind _output_get (`self.ChecklimitsrightStop`))
      (bind _output_get_2 (`self.Checklimitsleftstop`))
      (if (or _output_get _output_get_2)
        (set `self.speed` 0.0)
        (`self.AddMovementInput` (0.0 0.0 0.0))
        (else
          (`self.AddMovementInput` (`KismetMathLibrary.GetForwardVector` (`KismetMathLibrary.MakeRotator` 0.0 0.0 _returnvalue_yaw_2)))))
      (else
        (`self.Checklimitsright` :!label _label)
        (`self.Checklimitsleft`)
        (`self.AddMovementInput` (`KismetMathLibrary.GetForwardVector` (`KismetMathLibrary.MakeRotator` 0.0 0.0 _returnvalue_yaw)))))
    (else
      (set `self.speed` (`self.defaultSpeed`))
      (set `self.stop` false)
      (goto _label))))

(event `self.ReceiveActorBeginOverlap`
  (params (OtherActor :type "Actor Object Reference"))
  ;[1 1 1] Damage Main Character
  (bind _assoldier (cast `/Game/MyContent/Blueprints/MainCharacter/Soldier` OtherActor))
  (`/Game/MyContent/Blueprints/MainCharacter/Soldier.TakeDamage` _assoldier (`self.Damage`)))

(fn `CheckCharacter`
  (returns (Detected :type Boolean) (Character :type "/Game/MyContent/Blueprints/MainCharacter/Soldier Object Reference"))
  (bind _returnvalue (`self.K2_GetActorLocation`))
  (bind _outhits (`KismetSystemLibrary.SphereTraceMulti` :`Start` _returnvalue :`End` _returnvalue :`Radius` 500.0 :`TraceChannel` "TraceTypeQuery1" :`DrawDebugType` "ForOneFrame" :`bIgnoreSelf` false))
  (for _array_element _outhits
    (bind _assoldier (cast `/Game/MyContent/Blueprints/MainCharacter/Soldier` (`.HitActor` (`GameplayStatics.BreakHitResult` _array_element))))
    (return true _assoldier))
  (return false null))

(fn `Checklimitsleft`
  (bind (_origin _boxextent) (`KismetSystemLibrary.GetComponentBounds` (`self.CapsuleComponent`)))
  (bind _returnvalue (- (.z _origin) (.z _boxextent)))
  (bind _returnvalue_2 (- (.x _origin) (.x _boxextent)))
  (bind (_outhit _returnvalue_3) (`KismetSystemLibrary.LineTraceSingle` :`Start` (`KismetMathLibrary.MakeVector` _returnvalue_2 (.y _origin) _returnvalue) :`End` (`KismetMathLibrary.MakeVector` _returnvalue_2 (.y _origin) (- _returnvalue 50.0)) :`TraceChannel` "TraceTypeQuery1" :`DrawDebugType` "ForOneFrame"))
  (if (not _returnvalue_3)
    (set `self.speed` (* (`self.speed`) -1.0))
    (`self.K2_SetActorRotation` (struct))
    (set `self.isSwaped` false)))

(fn `Checklimitsleftstop`
  (returns (Output_Get :type Boolean))
  (bind (_origin _boxextent) (`KismetSystemLibrary.GetComponentBounds` (`self.CapsuleComponent`)))
  (bind _returnvalue (- (.z _origin) (.z _boxextent)))
  (bind _returnvalue_2 (- (.x _origin) (.x _boxextent)))
  (bind (_outhit _returnvalue_3) (`KismetSystemLibrary.LineTraceSingle` :`Start` (`KismetMathLibrary.MakeVector` _returnvalue_2 (.y _origin) _returnvalue) :`End` (`KismetMathLibrary.MakeVector` _returnvalue_2 (.y _origin) (- _returnvalue 50.0)) :`TraceChannel` "TraceTypeQuery1" :`DrawDebugType` "ForOneFrame"))
  (if _returnvalue_3
    (bind _output_get (set `self.stop` false))
    (return _output_get)
    (elif (`self.isSwaped`)
      (bind _output_get_2 (set `self.stop` true))
      (return _output_get_2)
      (else
        (bind _output_get_3 (set `self.stop` false))
        (return _output_get_3)))))

(fn `Checklimitsright`
  (bind (_origin _boxextent) (`KismetSystemLibrary.GetComponentBounds` (`self.CapsuleComponent`)))
  (bind _returnvalue (+ (.x _origin) (.x _boxextent)))
  (bind _returnvalue_2 (- (.z _origin) (.z _boxextent)))
  (bind (_outhit _returnvalue_3) (`KismetSystemLibrary.LineTraceSingle` :`Start` (`KismetMathLibrary.MakeVector` _returnvalue (.y _origin) _returnvalue_2) :`End` (`KismetMathLibrary.MakeVector` _returnvalue (.y _origin) (- _returnvalue_2 50.0)) :`TraceChannel` "TraceTypeQuery1" :`DrawDebugType` "ForOneFrame"))
  (if (not _returnvalue_3)
    (set `self.speed` (* (`self.speed`) -1.0))
    (`self.K2_SetActorRotation` (struct :`Yaw` 180.0))
    (set `self.isSwaped` true)))

(fn `ChecklimitsrightStop`
  (returns (Output_Get :type Boolean))
  (bind (_origin _boxextent) (`KismetSystemLibrary.GetComponentBounds` (`self.CapsuleComponent`)))
  (bind _returnvalue (+ (.x _origin) (.x _boxextent)))
  (bind _returnvalue_2 (- (.z _origin) (.z _boxextent)))
  (bind (_outhit _returnvalue_3) (`KismetSystemLibrary.LineTraceSingle` :`Start` (`KismetMathLibrary.MakeVector` _returnvalue (.y _origin) _returnvalue_2) :`End` (`KismetMathLibrary.MakeVector` _returnvalue (.y _origin) (- _returnvalue_2 50.0)) :`TraceChannel` "TraceTypeQuery1" :`DrawDebugType` "ForOneFrame"))
  (if _returnvalue_3
    (bind _output_get (set `self.stop` false))
    (return _output_get)
    (elif (`self.isSwaped`)
      (bind _output_get_2 (set `self.stop` false))
      (return _output_get_2)
      (else
        (bind _output_get_3 (set `self.stop` true))
        (return _output_get_3)))))

(fn `CheckVision`
  (params (Character :type "/Game/MyContent/Blueprints/MainCharacter/Soldier Object Reference"))
  (returns (Detected :type Boolean))
  (`/Engine/EditorBlueprintResources/StandardMacros.IsValid` Character
    (:`Is Valid`
      (bind _outhit (`KismetSystemLibrary.LineTraceSingle` :`Start` (`SceneComponent.K2_GetComponentLocation` (`self.Eyes`)) :`End` (`self.K2_GetActorLocation` Character) :`TraceChannel` "TraceTypeQuery1" :`DrawDebugType` "ForOneFrame" :`bIgnoreSelf` false))
      (cast `/Game/MyContent/Blueprints/MainCharacter/Soldier` (`.HitActor` (`GameplayStatics.BreakHitResult` _outhit))
        (:`then`
          (return true))
        (:`CastFailed`
          (return false))))))

(fn `GetDirection`
  (`/Engine/EditorBlueprintResources/StandardMacros.IsValid` (`self.CharacterReference`)
    (:`Is Valid`
      (set `self.Direction` (`KismetMathLibrary.Normal` (- (`SceneComponent.K2_GetComponentLocation` (`self.Mesh`)) (`self.K2_GetActorLocation`)))))))

(fn `UserConstructionScript`)