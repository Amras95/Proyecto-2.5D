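; Homing bullet actor that chases its Soldier target and deals damage on contact.
; Each Tick, GetDirection re-aims at the target with Z zeroed, keeping the last direction if the target is invalid, then the actor moves by Speed and delta time.
; Overlapping any Soldier calls TakeDamage with Damage and destroys the bullet, which otherwise destroys itself after a short BeginPlay delay.
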(event `self.ReceiveBeginPlay`
  (`KismetSystemLibrary.Delay` 1.0)
  (`/Engine/EditorBlueprintResources/StandardMacros.IsValid` self
    (:`Is Valid`
      (`self.K2_DestroyActor` self))))

(event `self.ReceiveTick`
  (params (DeltaSeconds :type "Float (single-precision)"))
  (bind (_returnvalue_x _returnvalue_y _returnvalue_z) (`KismetMathLibrary.BreakVector` (`self.K2_GetActorLocation`)))
  (bind (_direction_x _direction_y _direction_z) (`KismetMathLibrary.BreakVector` (`self.Direction`)))
  (bind (_returnvalue_x_2 _returnvalue_y_2 _returnvalue_z_2) (`KismetMathLibrary.BreakVector` (* DeltaSeconds (`self.Speed`))))
  (bind (_returnvalue_x_3 _returnvalue_y_3 _returnvalue_z_3) (`KismetMathLibrary.BreakVector` (* (`KismetMathLibrary.MakeVector` _direction_x _direction_y _direction_z) (`KismetMathLibrary.MakeVector` _returnvalue_x_2 _returnvalue_y_2 _returnvalue_z_2))))
  (bind (_returnvalue_x_4 _returnvalue_y_4 _returnvalue_z_4) (`KismetMathLibrary.BreakVector` (+ (`KismetMathLibrary.MakeVector` _returnvalue_x _returnvalue_y _returnvalue_z) (`KismetMathLibrary.MakeVector` _returnvalue_x_3 _returnvalue_y_3 _returnvalue_z_3))))
  (`self.GetDirection`)
  (`self.K2_SetActorLocation` (`KismetMathLibrary.MakeVector` _returnvalue_x_4 _returnvalue_y_4 _returnvalue_z_4)))

(event `self.ReceiveActorBeginOverlap`
  (params (OtherActor :type "Actor Object Reference"))
  (bind _assoldier (cast `/Game/MyContent/Blueprints/MainCharacter/Soldier` OtherActor))
  (`/Game/MyContent/Blueprints/MainCharacter/Soldier.TakeDamage` _assoldier (`self.Damage`))
  (`self.K2_DestroyActor`))

(fn `GetDirection`
  (bind (_returnvalue_x _returnvalue_y _returnvalue_z) (`KismetMathLibrary.BreakVector` (`self.K2_GetActorLocation`)))
  (bind _soldier (`self.Soldier`))
  (bind (_returnvalue_x_2 _returnvalue_y_2 _returnvalue_z_2) (`KismetMathLibrary.BreakVector` (`self.K2_GetActorLocation` _soldier)))
  (bind (_returnvalue_x_3 _returnvalue_y_3 _returnvalue_z_3) (`KismetMathLibrary.BreakVector` (- (`KismetMathLibrary.MakeVector` _returnvalue_x_2 _returnvalue_y_2 _returnvalue_z_2) (`KismetMathLibrary.MakeVector` _returnvalue_x _returnvalue_y _returnvalue_z))))
  (bind (_returnvalue_x_4 _returnvalue_y_4) (`KismetMathLibrary.BreakVector` (`KismetMathLibrary.Normal` (`KismetMathLibrary.MakeVector` _returnvalue_x_3 _returnvalue_y_3 _returnvalue_z_3))))
  (`/Engine/EditorBlueprintResources/StandardMacros.IsValid` _soldier
    (:`Is Valid`
      (set `self.Direction` (`KismetMathLibrary.MakeVector` _returnvalue_x_4 _returnvalue_y_4))
      (return))))

(fn `UserConstructionScript`)