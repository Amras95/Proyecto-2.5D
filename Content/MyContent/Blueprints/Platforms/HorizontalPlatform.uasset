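; HorizontalPlatform is a platform actor that moves back and forth along the world X axis.
; It records its start location on BeginPlay, then each Tick MoveHorizontal offsets X by Speed scaled by delta seconds.
; PingPongHorizontalCondition flags when X reaches either the start or start plus Distance, and Tick then negates Speed without clamping the position.
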(event `self.ReceiveBeginPlay`
  (set `self.Initialpos` (`self.K2_GetActorLocation`)))

(event `self.ReceiveTick`
  (params (DeltaSeconds :type "Float (single-precision)"))
  (`self.MoveHorizontal` 0.0)
  (if (`self.Ping pong horizontal condition`)
    (set `self.Speed` (* (`self.Speed`) -1.0))))

(fn `MoveHorizontal`
  (params (A :type "Float (double-precision)"))
  (bind (_returnvalue_x _returnvalue_y _returnvalue_z) (`KismetMathLibrary.BreakVector` (`self.K2_GetActorLocation`)))
  (`self.K2_SetActorLocation` (`KismetMathLibrary.MakeVector` (+ (* (`GameplayStatics.GetWorldDeltaSeconds`) (`self.Speed`)) _returnvalue_x) _returnvalue_y _returnvalue_z)))

(fn `Ping pong horizontal condition`
  (returns (ReturnValue :type Boolean))
  (bind _returnvalue_x (`KismetMathLibrary.BreakVector` (`self.K2_GetActorLocation`)))
  (bind _returnvalue_x_2 (`KismetMathLibrary.BreakVector` (`self.K2_GetActorLocation`)))
  (bind _initialpos_x (`KismetMathLibrary.BreakVector` (`self.Initialpos`)))
  (bind _initialpos_x_2 (`KismetMathLibrary.BreakVector` (`self.Initialpos`)))
  (return (or (<= (+ _initialpos_x (`self.Distance`)) _returnvalue_x_2) (>= _initialpos_x_2 _returnvalue_x))))

(fn `UserConstructionScript`)